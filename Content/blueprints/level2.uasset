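; Level transition trigger actor that loads Level4 when the player presses the level_change input while standing in its box.
; Box overlap events set an Overlaping flag only for BP_Sasha.
; The actor enables input on player controller 0 at BeginPlay, and the press opens the level after a short delay.
; PressedButton is set on press and never reset.
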(event `self.ReceiveBeginPlay`
  (`self.EnableInput` (`GameplayStatics.GetPlayerController` 0)))

(event `InputAction|level_change`
  (params (Key :type "Key Structure"))
  (:`Pressed`
    (set `self.pressed_button` true)
    (if (and (`self.pressed_button`) (`self.overlaping`))
      (`KismetSystemLibrary.Delay` 0.2)
      (`GameplayStatics.OpenLevel` "Level4"))))

(event `self.Box.OnComponentBeginOverlap`
  (params (OverlappedComponent :type "PrimitiveComponent Object Reference") (OtherActor :type "Actor Object Reference") (OtherComp :type "PrimitiveComponent Object Reference") (OtherBodyIndex :type Integer) (bFromSweep :type Boolean) (SweepResult :type "HitResult Structure (by ref)"))
  (cast `/Game/MetaHumans/Sasha/BP_Sasha` OtherActor)
  (set `self.overlaping` true))

(event `self.Box.OnComponentEndOverlap`
  (params (OverlappedComponent :type "PrimitiveComponent Object Reference") (OtherActor :type "Actor Object Reference") (OtherComp :type "PrimitiveComponent Object Reference") (OtherBodyIndex :type Integer))
  (cast `/Game/MetaHumans/Sasha/BP_Sasha` OtherActor)
  (set `self.overlaping` false))

(fn `UserConstructionScript`)