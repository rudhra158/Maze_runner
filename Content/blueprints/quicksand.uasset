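; Quicksand hazard Blueprint that traps BP_Sasha while the character overlaps its box.
; On entry it zeroes gravity, cuts horizontal velocity for a slow sinking motion, and sets a delayed timer for the character's dec_health function.
; On exit it sets Health to full and gravity to a fixed scale, without clearing the timer.
; Separately, a hit on Cube1 destroys that component after a short delay.
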(event `self.Box.OnComponentBeginOverlap`
  (params (OverlappedComponent :type "PrimitiveComponent Object Reference") (OtherActor :type "Actor Object Reference") (OtherComp :type "PrimitiveComponent Object Reference") (OtherBodyIndex :type Integer) (bFromSweep :type Boolean) (SweepResult :type "HitResult Structure (by ref)"))
  (bind _asbp_sasha (cast `/Game/MetaHumans/Sasha/BP_Sasha` OtherActor))
  (`KismetSystemLibrary.K2_SetTimer` _asbp_sasha "dec_health" 4.0)
  (bind _charactermovement (`Character.CharacterMovement` _asbp_sasha))
  (set `CharacterMovementComponent.GravityScale` 0.0 _charactermovement)
  (bind (_velocity_x _velocity_y) (`KismetMathLibrary.BreakVector` (`MovementComponent.Velocity` _charactermovement)))
  (set `MovementComponent.Velocity` (`KismetMathLibrary.MakeVector` (/ _velocity_x 6.0) (/ _velocity_y 6.0) -50.0) _charactermovement))

(event `self.Box.OnComponentEndOverlap`
  (params (OverlappedComponent :type "PrimitiveComponent Object Reference") (OtherActor :type "Actor Object Reference") (OtherComp :type "PrimitiveComponent Object Reference") (OtherBodyIndex :type Integer))
  (bind _asbp_sasha (cast `/Game/MetaHumans/Sasha/BP_Sasha` OtherActor))
  (set `self.health` 100)
  (set `CharacterMovementComponent.GravityScale` 1.5 (`Character.CharacterMovement` _asbp_sasha)))

(event `self.Cube1.OnComponentHit`
  (params (HitComponent :type "PrimitiveComponent Object Reference") (OtherActor :type "Actor Object Reference") (OtherComp :type "PrimitiveComponent Object Reference") (NormalImpulse :type "Vector Structure") (Hit :type "HitResult Structure (by ref)"))
  (`KismetSystemLibrary.Delay` 3.0)
  (`ActorComponent.K2_DestroyComponent` (`self.Cube1`)))

(fn `UserConstructionScript`)